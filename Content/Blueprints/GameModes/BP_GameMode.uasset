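; BP_GameMode is a game mode that runs endless waves of aliens with growing difficulty.
; Each wave multiplies WaveDifficulty to set the spawn count, then a looping named timer spawns BP_Alien actors at random TargetPoints until the count runs out.
; RegisterAlienDeath removes aliens from the tracked array and, once none remain alive or pending, ends the wave, starting the next after a short delay.
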(event Custom|Spawn%20Wave
  (CallFunction|SpawnAlien))

(event Custom|End%20Wave
  (Utilities|FlowControl|Delay 2.0)
  (CallFunction|StartNewWave))

(event EventBeginPlay
  (Utilities|FlowControl|Delay 2.0)
  (CallFunction|StartNewWave))

(fn ConstructionScript)

(fn StartNewWave
  (Math|Integer|IncrementInt (Variables|Default|GetCurrentWave)
    (:%20%20
      (CallFunction|IncreaseWaveDifficulty)
      (Utilities|Time|SetTimerbyFunctionName 0 "Spawn Wave" (Variables|Default|GetSpawnFrequency) true))))

(fn SpawnAlien
  (bind _spawnpoint (CallFunction|GetRandomSpawnPoint))
  (Utilities|IsValid _spawnpoint
    (:Is%20Valid
      (bind _returnvalue (Game|SpawnActorfromClass "/Game/Blueprints/AI/BP_Alien.BP_Alien_C" (Transformation|GetActorTransform _spawnpoint) "Undefined" 0 0))
      (Utilities|IsValid _returnvalue
        (:Is%20Valid
          (Utilities|Array|Add (Variables|Default|GetAliens) _returnvalue)
          (bind _result (Math|Integer|DecrementInt (Variables|Default|GetRemainingAlienSpawns))
            (:%20%20
              (if (== _result 0)
                (Utilities|Time|ClearTimerbyFunctionName 0 "Spawn Wave")))))))))

(fn GetRandomSpawnPoint
  (bind _outactors (Actor|GetAllActorsOfClass "/Script/Engine.TargetPoint"))
  (return (Utilities|Array|Get(acopy) _outactors (Math|Random|RandomIntegerinRange 0 (Utilities|Array|LastIndex _outactors)))))

(fn RegisterAlienDeath
  (params (Alien :type BP%20Alien%20Object%20Reference%20%28by%20ref%29))
  (Utilities|Array|RemoveItem (Variables|Default|GetAliens) Alien)
  (if (and (== (Utilities|Array|Length (Variables|Default|GetAliens)) 0) (== (Variables|Default|GetRemainingAlienSpawns) 0))
    (CallFunction|EndWave)))

(fn IncreaseWaveDifficulty
  (bind _output_get (Variables|Default|SetWaveDifficulty (Math|Float|Round (* (Variables|Default|GetWaveDifficulty) (Variables|Default|GetDifficultyMultiplier)))))
  (Variables|Default|SetRemainingAlienSpawns _output_get))