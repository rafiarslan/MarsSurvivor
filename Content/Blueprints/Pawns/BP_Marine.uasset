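; Player marine pawn for a shooter with world-axis movement, creating the HUD and handling health, death, kill count and pause menu.
; Aim sets control yaw from thumbstick direction or smoothed mouse velocity past deadzones, switching by the last key pressed.
; Firing loops sound and muzzle effect while a timer repeats line traces from the muzzle socket along control rotation, applying damage and impact effects.
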(event EventTick
  (params (DeltaSeconds :type Float%20%28single-precision%29))
  ;[1 1 1] Player Mouse/Controller Aim
  (if (CallFunction|IsPlayerAlive)
    (if (stale Input|KeyboardEvents|AnyKey _output_get)
      (ThumbstickInput|UpdateThumbstickAim)
      (else
        (MouseInput|UpdateMouseAim)))))

(event EventBeginPlay
  ;[1 1 1] Create Player HUD
  (bind _returnvalue (UserInterface|CreateWidget "/Game/UI/WBP_PlayerHUD.WBP_PlayerHUD_C" 0 self))
  (UserInterface|Viewport|AddtoViewport _returnvalue 0))

(event Game|Damage|EventAnyDamage
  (params (Damage :type Float%20%28single-precision%29) (DamageType :type Damage%20Type%20Object%20Reference) (InstigatedBy :type Controller%20Object%20Reference) (DamageCauser :type Actor%20Object%20Reference))
  ;[1 1 1] Stop Player Weapon Fire if Dead
  (if (CallFunction|IsPlayerAlive)
    (bind _output_get (Variables|PlayerProperties|SetPlayerHealth (Math|Float|Clamp(Float) (- (Variables|PlayerProperties|GetPlayerHealth) Damage) 0.0 1e+02)))
    (if (<= _output_get 0.0)
      (Variables|PlayerProperties|SetPlayerDead true)
      (CallFunction|StopWeaponFire))))

(event Input|ActionEvents|InputActionFireWeapon
  (params (Key :type Key%20Structure :default "None"))
  ;[1 1 1] Player Weapon Fire
  (:Pressed
    (CallFunction|StartWeaponFire))
  (:Released
    (CallFunction|StopWeaponFire)))

(event Input|ActionEvents|InputActionPauseGame
  (params (Key :type Key%20Structure :default "None"))
  (bind _returnvalue (Game|GetPlayerController 0))
  ;[1 1 1] Pause/Unpause Game
  (:Pressed
    (Utilities|IsValid (Variables|Default|GetPauseMenuReference)
      (:Is%20Valid
        _)
      (:Is%20Not%20Valid
        (bind _returnvalue_2 (UserInterface|CreateWidget "/Game/UI/WBP_PauseMenu.WBP_PauseMenu_C"))
        (Variables|Default|SetPauseMenuReference _returnvalue_2)))
    (if (Game|IsGamePaused)
      (Widget|RemovefromParent (Variables|Default|GetPauseMenuReference))
      (Game|SetGamePaused false)
      (Variables|/Script/Engine.PlayerController|SetbShowMouseCursor _returnvalue false)
      (Input|SetInputModeGameOnly _returnvalue)
      (else
        (UserInterface|Viewport|AddtoViewport (Variables|Default|GetPauseMenuReference) 0)
        (Game|SetGamePaused true)
        (Variables|/Script/Engine.PlayerController|SetbShowMouseCursor _returnvalue true)
        (Input|SetInputModeGameandUI _returnvalue (Variables|Default|GetPauseMenuReference) "LockInFullscreen" false)))))

(event Input|AxisEvents|InputAxisMoveForward/Backward
  (params (AxisValue :type Float%20%28single-precision%29))
  ;[1 1 1] Player Movement
  (if (CallFunction|IsPlayerAlive)
    (Pawn|Input|AddMovementInput "1.000000, 0, 0" AxisValue false)))

(event Input|AxisEvents|InputAxisMoveLeft/Right
  (params (AxisValue :type Float%20%28single-precision%29))
  ;[1 1 1] Player Movement
  (if (CallFunction|IsPlayerAlive)
    (Pawn|Input|AddMovementInput "0.000000,-1.000000, 0" AxisValue false)))

(event Input|KeyboardEvents|AnyKey
  (params (Key :type Key%20Structure :default "None"))
  ;[1 1 1] Player Mouse/Controller Aim
  (:Pressed
    (bind _output_get (Variables|ThumbstickInput|SetGamepadActive (Class|KismetInputLibrary|KeyIsGamepadKey Key)))))

(fn ConstructionScript)

(fn IsThumbstickAboveDeadzone
  (return (> (Math|Vector2D|Vector2DLength (Math|Vector2D|MakeVector2D (Input|AxisValues|GetThumbstickAimUp) (Input|AxisValues|GetThumbstickAimRight))) (Variables|ThumbstickInput|GetThumbstickDeadzone))))

(fn GetMouseVelocity
  (bind _returnvalue (Game|GetPlayerController 0))
  (bind (_deltax _deltay) (Class|PlayerController|GetInputMouseDelta _returnvalue))
  (return (/ (Math|Vector2D|MakeVector2D _deltax _deltay) (Utilities|Time|GetWorldDeltaSeconds))))

(fn IsMouseAboveDeadzone
  (return (> (Math|Vector2D|Vector2DLength (MouseInput|GetMouseVelocity)) (Variables|MouseInput|GetMouseDeadzone))))

(fn UpdateMouseAim
  (bind _returnvalue (Game|GetPlayerController 0))
  (bind _returnvalue_2 (MouseInput|GetMouseVelocity))
  (if (MouseInput|IsMouseAboveDeadzone)
    ;[1 1 1] Get mouse aim direction
    (Pawn|SetControlRotation _returnvalue (Math|Interpolation|RInterpTo (Pawn|GetControlRotation _returnvalue :!class /Script/Engine.Controller) (Math|Rotator|MakeRotator 0.0 0.0 (Class|KismetMathLibrary|DegAtan2 (.x _returnvalue_2) (.y _returnvalue_2))) (Utilities|Time|GetWorldDeltaSeconds) (Variables|MouseInput|GetMouseSmoothingStrength)))))

(fn UpdateThumbstickAim
  (if (ThumbstickInput|IsThumbstickAboveDeadzone)
    ;[1 1 1] Get thumbstick aim direction
    (Pawn|SetControlRotation (Game|GetPlayerController 0) (Math|Rotator|MakeRotator 0.0 0.0 (Class|KismetMathLibrary|DegAtan2 (Input|AxisValues|GetThumbstickAimRight) (Input|AxisValues|GetThumbstickAimUp))))))

(fn StartWeaponFire
  (if (CallFunction|IsPlayerAlive)
    (Components|Activation|Activate (Variables|Default|GetP_AssaultRifle_MF) false)
    (bind _returnvalue (Audio|SpawnSound2D "/Game/Sounds/Weapon_AssaultRifle/Stereo/RifleFireLoop_Cue.RifleFireLoop_Cue" 1.0 1.0 0.0 0))
    (Variables|Default|SetWeaponFireSound _returnvalue)
    (CallFunction|WeaponTrace)
    (Utilities|Time|SetTimerbyFunctionName 0 "WeaponTrace" (Variables|WeaponProperties|GetWeaponFireRate) true)))

(fn StopWeaponFire
  (Components|Activation|Deactivate (Variables|Default|GetP_AssaultRifle_MF))
  (Audio|Components|Audio|Stop (Variables|Default|GetWeaponFireSound))
  (Utilities|Time|ClearTimerbyFunctionName 0 "WeaponTrace")
  (if (CallFunction|IsPlayerAlive)
    (Audio|SpawnSound2D "/Game/Sounds/Weapon_AssaultRifle/Stereo/RifleFireEnd_Cue.RifleFireEnd_Cue" 1.0 1.0 0.0 0)))

(fn IsPlayerAlive
  (return (not (Variables|PlayerProperties|GetPlayerDead))))

(fn WeaponTrace
  (bind _outhit (Collision|LineTraceByChannel (CallFunction|GetWeaponTraceStartLocation) (CallFunction|GetWeaponTraceEndLocation) "TraceTypeQuery1" false 0 "None"))
  (if (.bBlockingHit (Collision|BreakHitResult _outhit))
    (Game|Damage|ApplyDamage (.HitActor (Collision|BreakHitResult _outhit)) (Variables|WeaponProperties|GetWeaponDamage) 0 0)
    (CallFunction|SpawnImpactHit (.Location (Collision|BreakHitResult _outhit)))))

(fn GetWeaponTraceStartLocation
  (return (Transformation|GetSocketLocation (Variables|Default|GetRifleMesh) "MuzzleFlashSocket")))

(fn GetWeaponTraceEndLocation
  (return (+ (CallFunction|GetWeaponTraceStartLocation) (* (Math|Vector|GetForwardVector (Pawn|GetControlRotation :!class /Script/Engine.Pawn)) (Variables|WeaponProperties|GetWeaponRange)))))

(fn IncreasePlayerKillCount
  (bind _result (Math|Integer|IncrementInt (Variables|PlayerProperties|GetPlayerKills))
    (:%20%20
      (Variables|PlayerProperties|SetPlayerKills _result))))

(fn SpawnImpactHit
  (params (HitLocation :type Vector))
  (Effects|SpawnEmitteratLocation "/Game/Effects/Weapons/Impacts/P_AssaultRifle_IH.P_AssaultRifle_IH" HitLocation))

(fn AddHealth
  (params (HealthToAdd :type Float%20%28single-precision%29))
  (Variables|PlayerProperties|SetPlayerHealth (Math|Float|Clamp(Float) (+ HealthToAdd (Variables|PlayerProperties|GetPlayerHealth)) 0.0 1e+02)))

(fn IsHealthFull
  (return (== (Variables|PlayerProperties|GetPlayerHealth) 1e+02)))